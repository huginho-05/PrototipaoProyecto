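; BP_VelocityBoost is a spinning pickup that temporarily changes the third-person character's max walk speed.
; Any overlap with its trigger hides it, disables collision and plays a ping at world origin, before the character cast.
; For that character, it saves the current speed, applies NewVelocity, then restores it after Duration, leaving the actor hidden rather than destroyed.
; Tick rotates the mesh by a fixed, frame-rate-dependent step.
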(event `self.PowerUpTrigger.OnComponentBeginOverlap`
  (params (OverlappedComponent :type "PrimitiveComponent Object Reference") (OtherActor :type "Actor Object Reference") (OtherComp :type "PrimitiveComponent Object Reference") (OtherBodyIndex :type Integer) (bFromSweep :type Boolean) (SweepResult :type "HitResult Structure (by ref)"))
  (`self.SetActorHiddenInGame` true)
  (`self.SetActorEnableCollision` false)
  (`GameplayStatics.PlaySoundAtLocation` "/Engine/EngineSounds/1kSineTonePing.1kSineTonePing" (0.0 0.0 0.0) (struct) 1.0 1.0 0.0 null null null null)
  (bind _asbp_third_person_character (cast `/Game/ThirdPerson/Blueprints/BP_ThirdPersonCharacter` OtherActor))
  (bind _charactermovement (`Character.CharacterMovement` _asbp_third_person_character))
  (set `self.OriginalVelocity` (`CharacterMovementComponent.MaxWalkSpeed` _charactermovement))
  (set `CharacterMovementComponent.MaxWalkSpeed` (`self.NewVelocity`) _charactermovement)
  (`KismetSystemLibrary.Delay` (`self.Duration`))
  (set `CharacterMovementComponent.MaxWalkSpeed` (`self.OriginalVelocity`) _charactermovement))

(event `self.ReceiveTick`
  (params (DeltaSeconds :type "Float (single-precision)"))
  (`SceneComponent.K2_AddLocalRotation` (`self.PowerUpMesh`) (struct :`Roll` 2.0) false false))

(fn `UserConstructionScript`)